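; GA_Reload is a Gameplay Ability that reloads the current weapon of BP_ThirdPersonCharacter.
; On activation it sets the character's Reloading flag and plays AM_Reload on the mesh.
; On montage completion it clears the flag, moves reserve Ammo into CurrentMag up to MagazineSize, clamped to what remains, then ends the ability.
; Only completion is handled, so an interrupted montage never reaches that cleanup.
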(event `self.K2_ActivateAbility`
  (`parent.K2_ActivateAbility`)
  (bind _asbp_third_person_character (cast `/Game/ThirdPerson/Blueprints/BP_ThirdPersonCharacter` (`self.GetAvatarActorFromActorInfo`)))
  (set `/Game/ThirdPerson/Blueprints/BP_ThirdPersonCharacter.Reloading` true _asbp_third_person_character)
  (`|PlayMontage` (`Character.Mesh` _asbp_third_person_character) "/Game/AnimStarterPack/UE5/AM_Reload.AM_Reload"
    (:`OnCompleted`
      (set `/Game/ThirdPerson/Blueprints/BP_ThirdPersonCharacter.Reloading` false _asbp_third_person_character)
      (bind _currentweapon (`/Game/ThirdPerson/Blueprints/BP_ThirdPersonCharacter.CurrentWeapon` _asbp_third_person_character))
      (bind _ammo (`/Game/Weapons/Pickups/BP_BaseWeapon.Ammo` _currentweapon))
      (set `self.TempAmmo` _ammo)
      (set `/Game/Weapons/Pickups/BP_BaseWeapon.Ammo` (`KismetMathLibrary.Clamp` (- _ammo (- (`/Game/Weapons/Pickups/BP_BaseWeapon.MagazineSize` _currentweapon) (`/Game/Weapons/Pickups/BP_BaseWeapon.CurrentMag` _currentweapon))) 0 (`/Game/Weapons/Pickups/BP_BaseWeapon.Ammo` _currentweapon)) _currentweapon)
      (set `/Game/Weapons/Pickups/BP_BaseWeapon.CurrentMag` (+ (- (`self.TempAmmo`) (`/Game/Weapons/Pickups/BP_BaseWeapon.Ammo` _currentweapon)) (`/Game/Weapons/Pickups/BP_BaseWeapon.CurrentMag` _currentweapon)) _currentweapon)
      (`self.K2_EndAbility`))))