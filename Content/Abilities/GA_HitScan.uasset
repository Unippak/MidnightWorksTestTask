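; Gameplay ability that fires one hitscan shot from the third-person character's current weapon, unless flagged out of ammo.
; AmmoCalculate decrements the clamped magazine count, and TraceCalculate supplies a line trace along the first-person camera's forward vector.
; The shot plays the pistol fire animation, then damages a hit Character or otherwise executes the Shot gameplay cue.
; An emptied magazine sends the Weapon.Reload gameplay event unless all ammo is gone, then the ability ends.
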(event `self.K2_ActivateAbility`
  (`parent.K2_ActivateAbility`)
  (if (`self.AmmoEmpty`)
    (`self.K2_EndAbility`)
    (else
      (bind _asbp_third_person_character (cast `/Game/ThirdPerson/Blueprints/BP_ThirdPersonCharacter` (`self.GetAvatarActorFromActorInfo`)))
      (bind _currentweapon (`/Game/ThirdPerson/Blueprints/BP_ThirdPersonCharacter.CurrentWeapon` _asbp_third_person_character))
      (bind _output_get (set `/Game/Weapons/Pickups/BP_BaseWeapon.CurrentMag` (`KismetMathLibrary.Clamp` (- (`/Game/Weapons/Pickups/BP_BaseWeapon.CurrentMag` _currentweapon) 1) 0 (`/Game/Weapons/Pickups/BP_BaseWeapon.MagazineSize` _currentweapon)) _currentweapon))
      (bind _firstpersoncamera (`/Game/ThirdPerson/Blueprints/BP_ThirdPersonCharacter.FirstPersonCamera` _asbp_third_person_character))
      (bind _returnvalue (`SceneComponent.K2_GetComponentLocation` _firstpersoncamera))
      (bind _outhit (`KismetSystemLibrary.LineTraceSingle` :`Start` _returnvalue :`End` (+ _returnvalue (* (`KismetMathLibrary.GetForwardVector` (`SceneComponent.K2_GetComponentRotation` _firstpersoncamera)) 10000.0)) :`TraceChannel` "TraceTypeQuery1" :`bIgnoreSelf` false))
      (set `self.AmmoEmpty` (and (== (`/Game/Weapons/Pickups/BP_BaseWeapon.Ammo` _currentweapon) 0) (== (`/Game/Weapons/Pickups/BP_BaseWeapon.CurrentMag` _currentweapon) 0)))
      (`SkeletalMeshComponent.PlayAnimation` _currentweapon "/Game/Packs/MilitaryWeapDark/Weapons/Anims/Fire_Pistol_W.Fire_Pistol_W" false)
      (bind (_bblockinghit _binitialoverlap _time _distance _location _impactpoint _normal _impactnormal _physmat _hitactor) (`GameplayStatics.BreakHitResult` _outhit))
      (bind _ascharacter (cast `Character` _hitactor)
        (:`then`
          (`GameplayStatics.ApplyDamage` _ascharacter 20.0))
        (:`CastFailed`
          (`GameplayCueFunctionLibrary.ExecuteGameplayCueOnActor` _hitactor (struct :`TagName` "GameplayCue.Shot") (`GameplayCueFunctionLibrary.MakeGameplayCueParametersFromHitResult` _outhit))))
      (if (== _output_get 0)
        (if (`self.AmmoEmpty`)
          (`self.K2_EndAbility`)
          (else
            (`AbilitySystemBlueprintLibrary.SendGameplayEventToActor` (`self.GetAvatarActorFromActorInfo`) (struct :`TagName` "Weapon.Reload"))
            (`self.K2_EndAbility`)))
        (else
          (`self.K2_EndAbility`))))))