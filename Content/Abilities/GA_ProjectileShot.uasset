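; Gameplay ability that fires a projectile from the third-person character's current weapon.
; Activation decrements the magazine count, clamped between zero and capacity, then spawns BP_Projectile at the Muzzle socket using the first-person camera's rotation.
; An empty magazine after the shot sends a Weapon.Reload gameplay event; otherwise a montage node runs, with the ability ending on either branch.
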(event `self.K2_ActivateAbility`
  (`parent.K2_ActivateAbility`)
  (bind _asbp_third_person_character (cast `/Game/ThirdPerson/Blueprints/BP_ThirdPersonCharacter` (`self.GetAvatarActorFromActorInfo`)))
  (bind _currentweapon (`/Game/ThirdPerson/Blueprints/BP_ThirdPersonCharacter.CurrentWeapon` _asbp_third_person_character))
  (bind _output_get (set `/Game/Weapons/Pickups/BP_BaseWeapon.CurrentMag` (`KismetMathLibrary.Clamp` (- (`/Game/Weapons/Pickups/BP_BaseWeapon.CurrentMag` _currentweapon) 1) 0 (`/Game/Weapons/Pickups/BP_BaseWeapon.MagazineSize` _currentweapon)) _currentweapon))
  (`|ExecutionSequence`
    (:`then_0`
      (bind (_returnvalue_location _returnvalue_rotation) (`KismetMathLibrary.BreakTransform` (`SceneComponent.K2_GetComponentToWorld` (`/Game/ThirdPerson/Blueprints/BP_ThirdPersonCharacter.FirstPersonCamera` _asbp_third_person_character))))
      (`|SpawnActorFromClass` "/Game/Weapons/Abilities/BP_Projectile.BP_Projectile_C" (`KismetMathLibrary.MakeTransform` (`SceneComponent.GetSocketLocation` _currentweapon "Muzzle") _returnvalue_rotation) "AdjustIfPossibleButAlwaysSpawn" "MultiplyWithRoot" null null)
      (if (== _output_get 0)
        (`AbilitySystemBlueprintLibrary.SendGameplayEventToActor` (`self.GetAvatarActorFromActorInfo`) (struct :`TagName` "Weapon.Reload"))
        (`self.K2_EndAbility`)
        (else
          (`|PlayMontage` null
            (:`then`
              (`self.K2_EndAbility`))))))))