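; GA_WallRun is a Gameplay Ability that forms an unfinished wall run, currently only probing for a wall beside the character.
; On activation it casts the avatar to Character and runs a debug-drawn Visibility line trace along its right vector, scaled by TraceDirection.
; It then ends immediately without using the hit; a yaw calculation from the hit normal is left unconnected.
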(event `self.K2_ActivateAbility`
  (`parent.K2_ActivateAbility`)
  (bind _ascharacter (cast `Character` (`self.GetAvatarActorFromActorInfo`)))
  (bind _returnvalue (`Actor.K2_GetActorLocation` _ascharacter))
  (bind _outhit (`KismetSystemLibrary.LineTraceSingle` :`Start` _returnvalue :`End` (+ _returnvalue (* (`Actor.GetActorRightVector` _ascharacter) (`self.TraceDirection`))) :`TraceChannel` "TraceTypeQuery1" :`DrawDebugType` "ForDuration"))
  (`self.K2_EndAbility`))