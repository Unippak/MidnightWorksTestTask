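; Gameplay ability for hitscan weapon fire on BP_ThirdPersonCharacter.
; On activation it decrements and prints the current weapon's ammo before checking it.
; With ammo left, it line-traces forward from the follow camera with debug drawing and executes a Shot gameplay cue on the hit actor, applying no damage.
; Otherwise it sends a Weapon.Reload event to the avatar without firing, and either path ends the ability.
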(event `self.K2_ActivateAbility`
  (`parent.K2_ActivateAbility`)
  (bind _asbp_third_person_character (cast `/Game/ThirdPerson/Blueprints/BP_ThirdPersonCharacter` (`self.GetAvatarActorFromActorInfo`)))
  (bind _currentweapon (`/Game/ThirdPerson/Blueprints/BP_ThirdPersonCharacter.CurrentWeapon` _asbp_third_person_character))
  (bind _output_get (set `/Game/Weapons/Pickups/BP_BaseWeapon.Ammo` (- (`/Game/Weapons/Pickups/BP_BaseWeapon.Ammo` _currentweapon) 1) _currentweapon))
  (`KismetSystemLibrary.PrintString` (`KismetStringLibrary.Conv_IntToString` _output_get))
  (if (<= 1 _output_get)
    (bind _followcamera (`/Game/ThirdPerson/Blueprints/BP_ThirdPersonCharacter.FollowCamera` _asbp_third_person_character))
    (bind _returnvalue (`SceneComponent.K2_GetComponentLocation` _followcamera))
    (bind _outhit (`KismetSystemLibrary.LineTraceSingle` :`Start` _returnvalue :`End` (+ _returnvalue (* (`KismetMathLibrary.GetForwardVector` (`SceneComponent.K2_GetComponentRotation` _followcamera)) 10000.0)) :`TraceChannel` "TraceTypeQuery1" :`DrawDebugType` "ForDuration"))
    (`GameplayCueFunctionLibrary.ExecuteGameplayCueOnActor` (`.HitActor` (`GameplayStatics.BreakHitResult` _outhit)) (struct :`TagName` "GameplayCue.Shot") (`GameplayCueFunctionLibrary.MakeGameplayCueParametersFromHitResult` _outhit))
    (`self.K2_EndAbility`)
    (else
      (`AbilitySystemBlueprintLibrary.SendGameplayEventToActor` (`self.GetAvatarActorFromActorInfo`) (struct :`TagName` "Weapon.Reload"))
      (`self.K2_EndAbility`))))