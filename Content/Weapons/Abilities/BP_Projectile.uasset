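; Weapon projectile actor that plays a non-spatial grenade launcher fire sound on spawn and destroys itself after a short lifetime.
; Sphere overlap applies point damage to the sweep result's hit actor, passing the sweep location as the hit direction, then destroys the projectile.
; Static mesh hit fires the GameplayCue.Projectile cue once on itself with parameters built from the hit result, then destroys the projectile.
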(event `self.ReceiveBeginPlay`
  (`GameplayStatics.PlaySound2D` "/Game/MilitaryWeapDark/Sound/GrenadeLauncher/Wavs/GrenadeLauncherB_Fire_ST02.GrenadeLauncherB_Fire_ST02" 1.0 1.0 0.0 null null)
  (`KismetSystemLibrary.Delay` 5.0)
  (`self.K2_DestroyActor`))

(event `self.Sphere.OnComponentBeginOverlap`
  (params (OverlappedComponent :type "PrimitiveComponent Object Reference") (OtherActor :type "Actor Object Reference") (OtherComp :type "PrimitiveComponent Object Reference") (OtherBodyIndex :type Integer) (bFromSweep :type Boolean) (SweepResult :type "HitResult Structure (by ref)"))
  (bind (_bblockinghit _binitialoverlap _time _distance _location _impactpoint _normal _impactnormal _physmat _hitactor) (`GameplayStatics.BreakHitResult` SweepResult))
  (`|ExecutionSequence`
    (:`then_0`
      (`GameplayStatics.ApplyPointDamage` _hitactor 2.0 _location SweepResult))
    (:`then_1`
      (`self.K2_DestroyActor`))))

(event `self.StaticMesh.OnComponentHit`
  (params (HitComponent :type "PrimitiveComponent Object Reference") (OtherActor :type "Actor Object Reference") (OtherComp :type "PrimitiveComponent Object Reference") (NormalImpulse :type "Vector Structure") (Hit :type "HitResult Structure (by ref)"))
  (`|ExecutionSequence`
    (:`then_0`
      (`/Engine/EditorBlueprintResources/StandardMacros.DoOnce` false
        (:`Completed`
          (`GameplayCueFunctionLibrary.ExecuteGameplayCueOnActor` self (struct :`TagName` "GameplayCue.Projectile") (`GameplayCueFunctionLibrary.MakeGameplayCueParametersFromHitResult` Hit)))))
    (:`then_1`
      (`self.K2_DestroyActor`))))

(fn `UserConstructionScript`)