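; GA_ProjectileShot is a gameplay ability that fires a projectile from the player's current weapon.
; On activation it decrements and prints the weapon's ammo, then spawns BP_Projectile at the first-person camera transform if at least one round remains after decrementing.
; Otherwise it sends a Weapon.Reload gameplay event to the avatar; both paths end the ability.
; A disconnected todo branch sketches a line-of-sight-checked, target-aimed shot with a blackboard flag.
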(event `self.K2_ActivateAbility`
  (`parent.K2_ActivateAbility`)
  (bind _asbp_third_person_character (cast `/Game/ThirdPerson/Blueprints/BP_ThirdPersonCharacter` (`self.GetAvatarActorFromActorInfo`)))
  (bind _currentweapon (`/Game/ThirdPerson/Blueprints/BP_ThirdPersonCharacter.CurrentWeapon` _asbp_third_person_character))
  (bind _output_get (set `/Game/Weapons/Pickups/BP_BaseWeapon.Ammo` (- (`/Game/Weapons/Pickups/BP_BaseWeapon.Ammo` _currentweapon) 1) _currentweapon))
  (`KismetSystemLibrary.PrintString` (`KismetStringLibrary.Conv_IntToString` _output_get))
  (if (<= 1 _output_get)
    (`|SpawnActorFromClass` "/Game/Weapons/Abilities/BP_Projectile.BP_Projectile_C" (`SceneComponent.K2_GetComponentToWorld` (`/Game/ThirdPerson/Blueprints/BP_ThirdPersonCharacter.FirstPersonCamera` _asbp_third_person_character)) "AdjustIfPossibleButAlwaysSpawn" "MultiplyWithRoot" null null)
    (`self.K2_EndAbility`)
    (else
      (`AbilitySystemBlueprintLibrary.SendGameplayEventToActor` (`self.GetAvatarActorFromActorInfo`) (struct :`TagName` "Weapon.Reload"))
      (`self.K2_EndAbility`))))