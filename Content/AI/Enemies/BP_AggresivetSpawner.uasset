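; BP_AggresivetSpawner is a spawner actor that keeps an aggressive enemy bot in play by replacing it after it dies.
; On BeginPlay it spawns a BP_AggresivBot at its own location and hands it the spawner's patrol route.
; It binds to the bot's health component depletion event, which waits a respawn delay, then loops back into the same spawn logic so each replacement is wired identically.
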(event `self.ReceiveBeginPlay`
  (bind _returnvalue (`|SpawnActorFromClass` "/Game/AI/Enemies/Aggressive/BP_AggresivBot.BP_AggresivBot_C" (`KismetMathLibrary.Conv_VectorToTransform` (`self.K2_GetActorLocation`)) "Undefined" "MultiplyWithRoot" null null null :!label _label))
  (set `/Game/AI/Enemies/Aggressive/BP_AggresivBot.PatroleRoute` (`self.PatrolRoute`) _returnvalue)
  (bind _returnvalue_2 (`self.GetComponentByClass` _returnvalue "/Engine/EditorBlueprintResources/BP_HealthComponent.BP_HealthComponent_C"))
  (`/Engine/EditorBlueprintResources/StandardMacros.IsValid` _returnvalue_2
    (:`Is Valid`
      (add `/Engine/EditorBlueprintResources/BP_HealthComponent.OnHealthDepleted` _returnvalue_2 (delegate `SpawnBot`)))))

(event `SpawnBot`
  (`KismetSystemLibrary.Delay` (`self.RespawnDelay`))
  (goto _label))

(fn `UserConstructionScript`)