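; Patrol route Blueprint for aggressive enemy AI that defines waypoints as the points of its PatrolRoute spline.
; IncrementParolRoute steps PatrolIndex by Direct, flipping the direction at the first and last points so the route runs back and forth.
; GetSplinePointPosition returns the current point's world location.
; The index and direction live on the route itself rather than on whatever follows it.
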(event `IncrementParolRoute`
  (bind _output_get (set `self.PatrolIndex` (+ (`self.PatrolIndex`) (`self.Direct`))))
  (if (== _output_get (- (`SplineComponent.GetNumberOfSplinePoints` (`self.PatrolRoute`)) 1))
    (set `self.Direct` -1)
    (elif (== (`self.PatrolIndex`) 0)
      (set `self.Direct` 1))))

(fn `GetSplinePointPosition`
  (returns (Location :type "Vector Structure"))
  (return (`SplineComponent.GetLocationAtSplinePoint` (`self.PatrolRoute`) (`self.PatrolIndex`) "World")))

(fn `UserConstructionScript`)