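; Gameplay ability that lets the third-person character climb surfaces it faces.
; On activation it caches the avatar and starts a looping timer that sphere-traces a short distance forward.
; A hit switches movement to Flying, sets the Climbing flag and turns the character into the surface using the hit normal.
; A miss restores Walking and movement-oriented rotation, clears the flag and ends the ability.
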(event `Timer`
  (bind _returnvalue (`Actor.K2_GetActorLocation` (stale `self.K2_ActivateAbility` _asbp_third_person_character)))
  (bind (_outhit _returnvalue_2) (`KismetSystemLibrary.SphereTraceSingle` :`Start` _returnvalue :`End` (+ _returnvalue (* (`Actor.GetActorForwardVector` (stale `self.K2_ActivateAbility` _asbp_third_person_character)) 44.0)) :`Radius` 6.0 :`TraceChannel` "TraceTypeQuery1" :`DrawDebugType` "ForDuration"))
  (if _returnvalue_2
    (bind _charactermovement (`Character.CharacterMovement` (stale `self.K2_ActivateAbility` _asbp_third_person_character)))
    (`CharacterMovementComponent.SetMovementMode` _charactermovement "MOVE_Flying" 0)
    (set `CharacterMovementComponent.bOrientRotationToMovement` false _charactermovement)
    (set `/Game/ThirdPerson/Blueprints/BP_ThirdPersonCharacter.Climbing` true (stale `self.K2_ActivateAbility` _asbp_third_person_character))
    (bind (_returnvalue_roll _returnvalue_pitch _returnvalue_yaw) (`KismetMathLibrary.BreakRotator` (`KismetMathLibrary.MakeRotFromX` (`.Normal` (`GameplayStatics.BreakHitResult` _outhit)))))
    (`Actor.K2_SetActorRotation` (stale `self.K2_ActivateAbility` _asbp_third_person_character) (`KismetMathLibrary.MakeRotator` 0.0 0.0 (+ _returnvalue_yaw 180.0)) false)
    (else
      (`CharacterMovementComponent.SetMovementMode` _charactermovement "MOVE_Walking" 0)
      (set `CharacterMovementComponent.bOrientRotationToMovement` true _charactermovement)
      (set `/Game/ThirdPerson/Blueprints/BP_ThirdPersonCharacter.Climbing` false (stale `self.K2_ActivateAbility` _asbp_third_person_character))
      (`self.K2_EndAbility`))))

(event `self.K2_ActivateAbility`
  (`parent.K2_ActivateAbility`)
  (`|ExecutionSequence`
    (:`then_0`
      (bind _asbp_third_person_character (cast `/Game/ThirdPerson/Blueprints/BP_ThirdPersonCharacter` (`self.GetAvatarActorFromActorInfo`))))
    (:`then_1`
      (`KismetSystemLibrary.K2_SetTimerDelegate` (delegate `Timer`) 0.1 true))))