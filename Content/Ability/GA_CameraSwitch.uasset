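; Gameplay ability that switches the third-person character between its follow camera and first-person camera.
; On activation it casts the avatar to BP_ThirdPersonCharacter, then a FlipFlop alternates which camera component is active.
; Controller yaw rotation is enabled for first person and disabled for third person, and the ability ends after each switch.
; The toggle state lives in the FlipFlop node, not read from the cameras.
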(event `self.K2_ActivateAbility`
  (`parent.K2_ActivateAbility`)
  (bind _asbp_third_person_character (cast `/Game/ThirdPerson/Blueprints/BP_ThirdPersonCharacter` (`self.GetAvatarActorFromActorInfo`)))
  (`/Engine/EditorBlueprintResources/StandardMacros.FlipFlop`
    (:`A`
      (bind _followcamera (`/Game/ThirdPerson/Blueprints/BP_ThirdPersonCharacter.FollowCamera` _asbp_third_person_character))
      (`ActorComponent.SetActive` _followcamera false false)
      (set `Pawn.bUseControllerRotationYaw` true _asbp_third_person_character)
      (bind _firstpersoncamera (`/Game/ThirdPerson/Blueprints/BP_ThirdPersonCharacter.FirstPersonCamera` _asbp_third_person_character))
      (`ActorComponent.SetActive` _firstpersoncamera true false)
      (`self.K2_EndAbility`))
    (:`B`
      (`ActorComponent.SetActive` _followcamera true false)
      (set `Pawn.bUseControllerRotationYaw` false _asbp_third_person_character)
      (`ActorComponent.SetActive` _firstpersoncamera false false)
      (`self.K2_EndAbility`))))